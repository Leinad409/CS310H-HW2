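; BP_Target is a shootable target that tracks level completion when hit by a BP_FirstPersonProjectile.
; Each hit increments TargetsHit on the player's BP_FirstPersonCharacter and destroys the target, unless the count equals TotalTargets.
; On that final hit it opens LV_Level2.
; The level-name check is disconnected and the branch is hardwired true, so the LV_MainMenu path never runs.
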(event Collision|EventHit
  (params (MyComp :type Primitive%20Component%20Object%20Reference) (Other :type Actor%20Object%20Reference) (OtherComp :type Primitive%20Component%20Object%20Reference) (bSelfMoved :type Boolean) (HitLocation :type Vector :default "0, 0, 0") (HitNormal :type Vector :default "0, 0, 0") (NormalImpulse :type Vector :default "0, 0, 0") (Hit :type Hit%20Result%20Structure%20%28by%20ref%29))
  (Utilities|Casting|CastToBP_FirstPersonProjectile Other)
  (bind _asbp_first_person_character (Utilities|Casting|CastToBP_FirstPersonCharacter (Game|GetPlayerCharacter 0)))
  (Variables|/Game/FirstPerson/Blueprints/BP_FirstPersonCharacter.BP_FirstPersonCharacter_C|SetTargetsHit _asbp_first_person_character (+ (Variables|/Game/FirstPerson/Blueprints/BP_FirstPersonCharacter.BP_FirstPersonCharacter_C|GetTargetsHit _asbp_first_person_character) 1))
  (if (== (Variables|/Game/FirstPerson/Blueprints/BP_FirstPersonCharacter.BP_FirstPersonCharacter_C|GetTargetsHit _asbp_first_person_character) (Variables|/Game/FirstPerson/Blueprints/BP_FirstPersonCharacter.BP_FirstPersonCharacter_C|GetTotalTargets _asbp_first_person_character))
    (bind _returnvalue (Game|GetCurrentLevelName true))
    (if true
      (Game|OpenLevel(byObjectReference) "/Game/Levels/LV_Level2.LV_Level2")
      (else
        (Game|OpenLevel(byObjectReference) "/Game/Levels/LV_MainMenu.LV_MainMenu")))
    (else
      (Actor|DestroyActor))))

(fn ConstructionScript)